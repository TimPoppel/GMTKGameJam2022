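; Short-lived enemy action actor that resolves a block from the Enemy's dice roll as soon as it begins play.
; Critical failure gives zero, critical success multiplies MaxBlock by the crit variable, and other rolls give a rounded percentage of MaxBlock.
; It reports the block through EnemyActionMessage to the first BPI_TurnManaging actor found, then destroys itself.
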(event `self.ReceiveBeginPlay`
  (bind _enemy (`self.Enemy`))
  (`parent.ReceiveBeginPlay`)
  (set `self.Block` 0)
  (if (`/Game/Blueprints/Enemy/BP_BaseEnemy.Critical Failure` _enemy)
    (set `self.Block` 0)
    (elif (`/Game/Blueprints/Enemy/BP_BaseEnemy.Critical Success` _enemy)
      (set `self.Block` (* (`self.MaxBlock`) (`/Game/Blueprints/Enemy/BP_BaseEnemy.Crit Variable` _enemy)))
      (else
        (set `self.Block` (`KismetMathLibrary.Round` (* (`/Game/Blueprints/Enemy/BP_BaseEnemy.PercentageOutcome` _enemy) (`self.MaxBlock`)))))))
  (`self.SendActionData` 0 0 (`self.Block`))
  (`self.K2_DestroyActor`))

(fn `UserConstructionScript`
  (`parent.UserConstructionScript`))