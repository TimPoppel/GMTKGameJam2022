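; BP_EnemyBigAttack is a short-lived enemy attack actor that works out the damage of a big attack from the enemy's roll results.
; On BeginPlay it runs the parent logic, then sets Damage to zero on critical failure, crit-multiplied maximum on critical success, or otherwise a rounded percentage of maximum.
; It destroys itself immediately afterward without applying the damage in this graph, and its debug print chain is disconnected.
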(event `self.ReceiveBeginPlay`
  (bind _enemy (`self.Enemy`))
  (`parent.ReceiveBeginPlay`)
  (if (`/Game/Blueprints/Enemy/BP_BaseEnemy.Critical Failure` _enemy)
    (set `self.Damage` 0)
    (elif (`/Game/Blueprints/Enemy/BP_BaseEnemy.Critical Success` _enemy)
      (set `self.Damage` (* (`self.MaxDamage`) (`/Game/Blueprints/Enemy/BP_BaseEnemy.Crit Variable` _enemy)))
      (else
        (set `self.Damage` (`KismetMathLibrary.Round` (* (`/Game/Blueprints/Enemy/BP_BaseEnemy.PercentageOutcome` _enemy) (`self.MaxDamage`)))))))
  (`self.K2_DestroyActor`))

(fn `UserConstructionScript`
  (`parent.UserConstructionScript`))