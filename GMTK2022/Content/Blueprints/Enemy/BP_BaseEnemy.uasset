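; Base enemy for dice-driven turn combat that tracks health and telegraphs and performs abilities through the HUD.
; Buttonpressed rolls the dice component and picks a random ability, repeating both until it differs from the last two used.
; PerformAction plays ability feedback, converts non-critical rolls to a fraction of die size, then spawns the ability actor.
; Death notifies the turn manager interface before destroying itself; ability cooldown logic is present but unconnected.
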(event `self.ReceiveBeginPlay`
  (bind _hud_ref (`self.HUD ref`))
  (set `self.Health` (`self.MaxHealth`))
  (message `/Game/UI/PlayerUI/BPI_HudInterface.UpdateEnemyHealth` _hud_ref (`self.Health`) (`self.MaxHealth`))
  (`/Game/UI/PlayerUI/BPI_HudInterface.UpdateEnemyInformation` _hud_ref (`self.Image`) (`self.EnemyName`)))

(event `PerformAction`
  (bind _hud_ref (`self.HUD ref`))
  (bind _hud_ref_2 (`self.HUD ref`))
  (bind _hud_ref_3 (`self.HUD ref`))
  (bind _hud_ref_4 (`self.HUD ref`))
  (bind _hud_ref_5 (`self.HUD ref`))
  (bind _output (`|GetArrayItem` (`self.Abilities`) (`self.UsedAbility`)))
  (`|ExecutionSequence`
    (:`then_0`
      (if (== _output "/Game/Blueprints/Enemy/BP_EnemyBigAttack.BP_EnemyBigAttack_C")
        (`UserWidget.PlayAnimation` _hud_ref_3 (`/Game/UI/EnemyUI/WBP_Enemy.EnemyStrongAttack` _hud_ref_3) 0.0 1 "Forward" 1.0 false)
        (`GameplayStatics.PlaySound2D` "/Game/Sound/Enemy/A_EnemyHit_Cue.A_EnemyHit_Cue" 1.0 1.0 0.0 null null)
        (elif (== _output "/Game/Blueprints/Enemy/BP_EnemyBasicAttack.BP_EnemyBasicAttack_C")
          (`UserWidget.PlayAnimation` _hud_ref_5 (`/Game/UI/EnemyUI/WBP_Enemy.EnemyAttack` _hud_ref_5) 0.0 1 "Forward" 1.0 false)
          (`GameplayStatics.PlaySound2D` "/Game/Sound/Enemy/A_EnemyHitBig_Cue.A_EnemyHitBig_Cue" 1.0 1.0 0.0 null null)
          (elif (== (`|GetArrayItem` (`self.Abilities`) (`self.UsedAbility`)) "/Game/Blueprints/Enemy/BP_EnemyBlock.BP_EnemyBlock_C")
            (`UserWidget.PlayAnimation` _hud_ref_4 (`/Game/UI/EnemyUI/WBP_Enemy.EnemyBlock` _hud_ref_4) 0.0 1 "Forward" 1.0 false)
            (else
              (`UserWidget.PlayAnimation` _hud_ref (`/Game/UI/EnemyUI/WBP_Enemy.EnemyDodge` _hud_ref) 0.0 1 "Forward" 1.0 false))))))
    (:`then_1`
      (message `/Game/UI/PlayerUI/BPI_HudInterface.UpdateRolledTypeEnemy` _hud_ref_2 (`self.Dice Type`))
      (set `/Game/UI/EnemyUI/WBP_Enemy.Outcome Enemy` (`self.Dice Outcome`) _hud_ref_2)
      (if (`self.Critical Success`)
        _
        (elif (not (`self.Critical Failure`))
          (set `self.PercentageOutcome` (/ (`KismetMathLibrary.Conv_IntToDouble` (`self.Dice Outcome`)) (`KismetMathLibrary.Conv_IntToDouble` (`KismetStringLibrary.Conv_StringToInt` (`KismetStringLibrary.Replace` (`|GetEnumeratorNameAsString` (`self.Dice Type`)) "d")))))))
      (`|SpawnActorFromClass` (`|GetArrayItem` (`self.Abilities`) (`self.UsedAbility`)) (`KismetMathLibrary.MakeTransform` (0.0 0.0 0.0)) "Undefined" "OverrideRootScale" null self null))))

(event `Button pressed`
  (bind _bpc_dice (`self.BPC_Dice`))
  (`/Game/Blueprints/Components/DiceComponent/BPC_Dice.ShapeShiftDice` _bpc_dice 0)
  (bind (_diceoutcome _bcriticalsuccess _bcriticalfail _dicetype) (`/Game/Blueprints/Components/DiceComponent/BPC_Dice.RollDice` _bpc_dice 0 :!label _label))
  (set `self.Dice Outcome` _diceoutcome)
  (set `self.Critical Success` _bcriticalsuccess)
  (set `self.Critical Failure` _bcriticalfail)
  (bind _output_get (set `self.Dice Type` _dicetype))
  (message `/Game/UI/PlayerUI/BPI_HudInterface.UpdateDiceTypeEnemy` (`self.HUD ref`) _output_get)
  (bind _output_get_2 (set `self.RandomInteger` (`KismetMathLibrary.RandomInteger` (`KismetArrayLibrary.Array_Length` (`self.Abilities`)))))
  (if (or (== (`self.RandomInteger`) (`self.UsedAbility`)) (== (`self.RandomInteger`) (`self.UsedAbility2`)))
    (goto _label)
    (else
      (set `self.UsedAbility2` (`self.UsedAbility`))
      (set `self.UsedAbility` _output_get_2)
      (message `/Game/UI/PlayerUI/BPI_HudInterface.UpdateEnemyAction` (`self.HUD ref`) (`BlueprintMapLibrary.Map_Find` (`self.AbilityNames`) (`|GetArrayItem` (`self.Abilities`) (`self.UsedAbility`)))))))

(event `Take Damage`
  (params (DamageAmount :type Integer))
  (bind _returnvalue (- (`self.Health`) DamageAmount))
  (if (> DamageAmount 0)
    (`GameplayStatics.PlaySound2D` "/Game/Sound/Enemy/A_EnemyHurt_Cue.A_EnemyHurt_Cue" 1.0 1.0 0.0 null null))
  (if (> _returnvalue (`self.MaxHealth`))
    (set `self.Health` (`self.MaxHealth`))
    (else
      (set `self.Health` _returnvalue)))
  (message `/Game/UI/PlayerUI/BPI_HudInterface.UpdateEnemyHealth` (`self.HUD ref`) (`self.Health`) (`self.MaxHealth`))
  (if (<= (`self.Health`) 0)
    (`self.Death`)))

(event `Death`
  (bind _outactors (`GameplayStatics.GetAllActorsWithInterface` "/Game/Blueprints/TurnManager/BPI_TurnManaging.BPI_TurnManaging_C"))
  (message `/Game/Blueprints/TurnManager/BPI_TurnManaging.Died` (`|GetArrayItem` _outactors) self)
  (`KismetSystemLibrary.Delay` 0.2)
  (`/Game/UI/PlayerUI/BPI_HudInterface.UpdateEnemyInformation` (`self.HUD ref`) null "")
  (`self.K2_DestroyActor`))

(fn `UserConstructionScript`)