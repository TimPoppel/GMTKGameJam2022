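; BP_EnemyBasicAttack is a short-lived actor that resolves an enemy's basic attack from a dice outcome.
; On BeginPlay it sets damage to zero on critical failure, MaxDamage times the enemy's crit multiplier on critical success, or MaxDamage scaled by the outcome percentage otherwise.
; It sends the damage through EnemyActionMessage with no heal or block, then destroys itself.
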(event `self.ReceiveBeginPlay`
  (bind _enemy (`self.Enemy`))
  (`parent.ReceiveBeginPlay`)
  (set `self.Damage` 0)
  (if (`/Game/Blueprints/Enemy/BP_BaseEnemy.Critical Failure` _enemy)
    (set `self.Damage` 0)
    (elif (`/Game/Blueprints/Enemy/BP_BaseEnemy.Critical Success` _enemy)
      (set `self.Damage` (* (`self.MaxDamage`) (`/Game/Blueprints/Enemy/BP_BaseEnemy.Crit Variable` _enemy)))
      (else
        (set `self.Damage` (`KismetMathLibrary.Round` (* (`/Game/Blueprints/Enemy/BP_BaseEnemy.PercentageOutcome` _enemy) (`self.MaxDamage`)))))))
  (message `/Game/Blueprints/TurnManager/BPI_TurnManaging.EnemyAction` (`self.Damage`))
  (`self.K2_DestroyActor`))

(fn `UserConstructionScript`
  (`parent.UserConstructionScript`))