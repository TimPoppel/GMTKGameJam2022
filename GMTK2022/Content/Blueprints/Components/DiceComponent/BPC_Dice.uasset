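; BPC_Dice is a dice component that rolls dice from DiceInventory and can change shape-shift dice into a random new type.
; RollDice derives the maximum from the dice type enum's name by stripping the "d", flagging the top roll as a critical success and 1 as a critical fail.
; RollAndShapeShift rolls first, then calls ShapeShiftDice, which overwrites eligible inventory entries, and returns both rolled and shifted types.
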(fn `RollAndShapeShift`
  (params (DiceIndex :type Integer))
  (returns (DiceOutcome :type Integer) (bCriticalSuccess :type Boolean) (bCriticalFailure :type Boolean) (bShapeShifted :type Boolean) (DiceType :type "/Game/Blueprints/Components/DiceComponent/E_DiceType Enum") (ShiftedDiceType :type "/Game/Blueprints/Components/DiceComponent/E_DiceType Enum"))
  (bind (_diceoutcome _bcriticalsuccess _bcriticalfail _dicetype) (`self.RollDice` DiceIndex))
  (bind (_bshapeshifted _shifteddice) (`self.ShapeShiftDice` (`local.DiceIndex`)))
  (return _diceoutcome _bcriticalsuccess _bcriticalfail _bshapeshifted _dicetype _shifteddice))

(fn `RollDice`
  (params (DiceIndex :type Integer))
  (returns (DiceOutcome :type Integer) (bCriticalSuccess :type Boolean) (bCriticalFail :type Boolean) (DiceType :type "/Game/Blueprints/Components/DiceComponent/E_DiceType Enum"))
  (locals (RolledNumber :type Integer) (NewLocalVar_0 :type String :default "Hello"))
  (bind (_output_bisshapeshiftdice _output_currentdice) (break `/Game/Blueprints/Components/DiceComponent/F_Dice` (`|GetArrayItem` (`self.DiceInventory`) DiceIndex)))
  (bind _returnvalue (`KismetStringLibrary.Conv_StringToInt` (`KismetStringLibrary.Replace` (`|GetEnumeratorNameAsString` _output_currentdice) "d")))
  (bind _output_get (set `local.RolledNumber` (`KismetMathLibrary.RandomIntegerInRange` 1 _returnvalue)))
  (return _output_get (== _returnvalue (`local.RolledNumber`)) (== (`local.RolledNumber`) 1) _output_currentdice))

(fn `ShapeShiftDice`
  (params (DiceIndex :type Integer))
  (returns (bShapeShifted :type Boolean) (ShiftedDice :type "/Game/Blueprints/Components/DiceComponent/E_DiceType Enum"))
  (locals (NewShapeShiftDice :type "/Game/Blueprints/Components/DiceComponent/F_Dice Structure") (DiceType :type "/Game/Blueprints/Components/DiceComponent/E_DiceType Enum"))
  (bind (_output_bisshapeshiftdice _output_currentdice) (break `/Game/Blueprints/Components/DiceComponent/F_Dice` (`|GetArrayItem` (`self.DiceInventory`) DiceIndex)))
  (if _output_bisshapeshiftdice
    (bind _output_get (set `local.DiceType` (cast `/Game/Blueprints/Components/DiceComponent/E_DiceType` (`KismetMathLibrary.Conv_IntToByte` (`KismetMathLibrary.RandomIntegerInRange` 0 5)))))
    (bind _output_get_2 (set `local.NewShapeShiftDice` (make `/Game/Blueprints/Components/DiceComponent/F_Dice` true _output_get)))
    (`KismetArrayLibrary.Array_Set` (`self.DiceInventory`) (`local.DiceIndex`) _output_get_2)
    (return true (`local.DiceType`))
    (else
      (return false _output_currentdice))))