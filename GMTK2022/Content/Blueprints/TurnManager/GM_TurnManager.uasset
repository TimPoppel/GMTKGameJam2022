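; Turn manager that runs turn-based combat waves between BP_Player and spawned enemies.
; StartCombat picks a DT_Waves row by VictoryCount and spawns its enemy; each turn triggers enemy intent and accepts two player actions.
; NextTurn gathers enemy actions, nets damage against block, then applies damage and healing (as negative damage) to player and first enemy.
; Enemy death advances the wave and shows WBP_Victory; player death resets progress, with WBP_Defeat creation left unconnected.
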(event `self.ReceiveBeginPlay`
  ;[1 1 1] Event beginplay
  (bind _asbp_player (cast `/Game/Blueprints/Player/BP_Player` (`GameplayStatics.GetPlayerPawn` 0)))
  (set `self.As BP Player` _asbp_player)
  (bind _returnvalue (`|CreateWidget` "/Game/UI/EnemyUI/WBP_Enemy.WBP_Enemy_C" null null))
  (bind _output_get (set `self.Enemy HUD Ref` _returnvalue))
  (`UserWidget.AddToViewport` _output_get 1)
  (`self.StartCombat`))

(event `StartCombat`
  ;[0 1 0.5901] Start Combat
  (`self.Reset Turn Count`)
  ;;[1 1 1] check what enemy to spawn
  (bind _row (`self.CheckWave`))
  ;;[1 1 1] Spawn enemy
  (`self.SpawnEnemy` _row)
  ;;[1 1 1] start turn
  (`self.StartTurn`))

(event `/Game/Blueprints/TurnManager/BPI_TurnManaging.Died`
  (params (Caster :type "Pawn Object Reference"))
  (bind _returnvalue (== Caster (`GameplayStatics.GetPlayerPawn` 0)))
  ;[1 0 0.1117] End Combat
  ;;[1 1 1] Enemy/player Died
  ;;[1 1 1] Did the player die?
  (if _returnvalue
    ;;[1 1 1] Show GameOver Screen
    (`self.Reset Victory`)
    (`GameplayStatics.PlaySound2D` "/Game/Sound/Game/A_Defeat_Cue.A_Defeat_Cue" 1.0 1.0 0.0 null null))
  (if (not _returnvalue)
    ;;[1 1 1] proceed wave count
    (`/Engine/EditorBlueprintResources/StandardMacros.IncrementInt` (`self.VictoryCount`)
      (:`  `
        (`KismetSystemLibrary.Delay` 0.3)
        ;;[1 1 1] Show reward Screen
        (bind _returnvalue_2 (`|CreateWidget` "/Game/UI/Popup/WBP_Victory.WBP_Victory_C" (`GameplayStatics.GetPlayerController` 0)))
        (`UserWidget.AddToViewport` _returnvalue_2 1)
        (`KismetSystemLibrary.Delay` 0.1)
        (`GameplayStatics.PlaySound2D` "/Game/Sound/Game/A_Victory_Cue.A_Victory_Cue" 1.0 1.0 0.0 null null)))))

(event `StartTurn`
  ;[1 1 1] StartTurn
  ;;[1 1 1] Show Enemy Intent
  (`self.StartEnemyTurn `))

(event `Next Turn`
  ;[1 1 1] Going to the next Turn
  ;;[1 1 1] Player ends their turn
  ;;[1 1 1] Resolve enemy outcome
  (`self.ResolveOutcomes`)
  ;;[1 1 1] set up next turn.
  (`self.Increase Turn Count`)
  (`self.ClearActionData`)
  ;;[1 1 1] Start next turn
  (`self.StartTurn`))

(event `Increase Turn Count`
  ;[1 1 1] Counters
  (`/Engine/EditorBlueprintResources/StandardMacros.IncrementInt` (`self.TurnCount`)
    (:`  `
      (set `self.PlayerActionAmount` 0))))

(event `ClearActionData`
  ;[1 1 1] Counters
  (`self.ClearPlayer&EnemyActionData`))

(event `Reset Turn Count`
  ;[1 1 1] Counters
  (set `self.TurnCount` 0)
  (set `self.PlayerActionAmount` 0))

(event `Reset Victory`
  ;[1 1 1] Counters
  (set `self.VictoryCount` 0)
  (set `self.PlayerActionAmount` 0))

(event `/Game/Blueprints/TurnManager/BPI_TurnManaging.EnemyAction`
  (params (Damage :type Integer) (Heal :type Integer) (Block :type Integer))
  (`self.EnemyActionData` Damage Heal Block))

(event `/Game/Blueprints/TurnManager/BPI_TurnManaging.PlayerAction`
  (params (Damage :type Integer) (Health :type Integer) (Block :type Integer))
  (if (not (>= (`self.PlayerActionAmount`) 2))
    (`self.PlayerActionData` Damage Health Block)
    (`/Engine/EditorBlueprintResources/StandardMacros.IncrementInt` (`self.PlayerActionAmount`))))

(fn `CheckWave`
  (returns (Row :type Name))
  (bind _outrownames (`DataTableFunctionLibrary.GetDataTableRowNames` "/Game/Blueprints/TurnManager/DT_Waves.DT_Waves"))
  (for (_array_element _array_index) _outrownames
    (if (== (`self.VictoryCount`) _array_index)
      (return _array_element))))

(fn `EnemyActionData`
  (params (EnemyDamage :type Integer) (EnemyHeal :type Integer) (EnemyBlock :type Integer))
  (set `self.EnemyDamage` (+ EnemyDamage (`self.EnemyDamage`)))
  (set `self.EnemyHeal` (+ EnemyHeal (`self.EnemyHeal`)))
  (set `self.EnemyBlock` (+ EnemyBlock (`self.EnemyBlock`))))

(fn `EnemyDamageVsPlayerBlock`
  (bind _output_get (set `self.EnemyDamage` (- (`self.EnemyDamage`) (`self.PlayerBlock`))))
  (if (<= _output_get 0)
    (set `self.PlayerBlock` (+ (`self.PlayerBlock`) (`self.EnemyDamage`)))
    (set `self.EnemyDamage` 0)
    (else
      (set `self.PlayerBlock` 0))))

(fn `Get Outcomes`
  ;[1 1 1] Tell enemies to perform action
  (bind _outactors (`GameplayStatics.GetAllActorsOfClass` "/Game/Blueprints/Enemy/BP_BaseEnemy.BP_BaseEnemy_C"))
  (for _array_element _outactors
    (`/Game/Blueprints/Enemy/BP_BaseEnemy.PerformAction` _array_element))
  (return))

(fn `PlayerActionData`
  (params (PlayerDamage :type Integer) (PlayerHeal :type Integer) (PlayerBlock :type Integer))
  (set `self.PlayerDamage` (+ PlayerDamage (`self.PlayerDamage`)))
  (set `self.PlayerHeal` (+ PlayerHeal (`self.PlayerHeal`)))
  (set `self.PlayerBlock` (+ PlayerBlock (`self.PlayerBlock`))))

(fn `PlayerDamageVsEnemyBlock`
  (bind _output_get (set `self.PlayerDamage` (- (`self.PlayerDamage`) (`self.EnemyBlock`))))
  (if (<= _output_get 0)
    (set `self.EnemyBlock` (+ (`self.EnemyBlock`) (`self.PlayerDamage`)))
    (set `self.PlayerDamage` 0)
    (else
      (set `self.EnemyBlock` 0))))

(fn `ResolveOutcomes`
  ;[1 1 1] Get remaining Data
  (`self.Get Outcomes`)
  ;[1 1 1] Calculate damage vs blocking
  (`self.PlayerDamageVsEnemyBlock`)
  (`self.EnemyDamageVsPlayerBlock`)
  ;[1 1 1] Heal player
  (`/Game/Blueprints/Player/BP_Player.Take Damage` (`self.As BP Player`) (* (`self.PlayerHeal`) -1))
  ;[1 1 1] Heal Enemy
  (bind _outactors (`GameplayStatics.GetAllActorsOfClass` "/Game/Blueprints/Enemy/BP_BaseEnemy.BP_BaseEnemy_C"))
  (bind _output (`|GetArrayItem` _outactors))
  (`/Game/Blueprints/Enemy/BP_BaseEnemy.Take Damage` _output (* (`self.EnemyHeal`) -1))
  ;[1 1 1] Damage Enemy
  (`/Game/Blueprints/Enemy/BP_BaseEnemy.Take Damage` _output (`self.PlayerDamage`))
  ;[1 1 1] Damage Player
  (`/Game/Blueprints/Player/BP_Player.Take Damage` (`self.As BP Player`) (`self.EnemyDamage`))
  (return))

(fn `SpawnEnemy`
  (params (Row :type Name))
  (bind _returnvalue (`|GetDataTableRow` "/Game/Blueprints/TurnManager/DT_Waves.DT_Waves" Row)
    (:`then`
      (bind _returnvalue_2 (`GameplayStatics.GetActorOfClass` "/Game/Blueprints/BP_TestActor.BP_TestActor_C"))
      (`|SpawnActorFromClass` :`Class` (`.Enemy1_7_6642BFCC4387AD3C794E9F9A3CCA6B2A` (break `/Game/Blueprints/TurnManager/F_Waves` _returnvalue)) :`SpawnTransform` (`self.GetTransform` _returnvalue_2) :`CollisionHandlingOverride` "Undefined" :`TransformScaleMethod` "OverrideRootScale" :`HUD ref` (`self.Enemy HUD Ref`) :`Instigator` null))))

(fn `StartEnemyTurn `
  (bind _outactors (`GameplayStatics.GetAllActorsOfClass` "/Game/Blueprints/Enemy/BP_BaseEnemy.BP_BaseEnemy_C"))
  (for _array_element _outactors
    (`/Game/Blueprints/Enemy/BP_BaseEnemy.Button pressed` _array_element))
  (return))

(fn `UserConstructionScript`)