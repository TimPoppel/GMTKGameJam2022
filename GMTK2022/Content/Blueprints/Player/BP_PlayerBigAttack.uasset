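; BP_PlayerBigAttack is a short-lived actor that resolves the damage of the player's big attack.
; On BeginPlay, after the parent logic, it sets Damage from the outcome variables: multiplied maximum on critical success, zero on critical failure, otherwise a rounded percentage of maximum.
; It only prints the result and then destroys itself, without applying damage to any target in this graph.
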(event `self.ReceiveBeginPlay`
  (`parent.ReceiveBeginPlay`)
  (if (`self.Critical Success`)
    (set `self.Damage` (* (`self.Max Damage`) (`self.Crit Multiplier`)))
    (elif (`self.Critical Failure`)
      (set `self.Damage` 0)
      (else
        (set `self.Damage` (`KismetMathLibrary.Round` (* (`self.Percentage Outcome`) (`self.Max Damage`)))))))
  (`KismetSystemLibrary.PrintString` (`KismetStringLibrary.Conv_IntToString` (`self.Damage`)))
  (`self.K2_DestroyActor`))

(fn `UserConstructionScript`
  (`parent.UserConstructionScript`))