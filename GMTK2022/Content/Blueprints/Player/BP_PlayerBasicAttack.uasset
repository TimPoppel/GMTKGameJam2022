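; BP_PlayerBasicAttack is a short-lived actor for the player's basic attack that reports the attack outcome as on-screen debug text.
; On BeginPlay it runs the parent logic, then branches on CriticalSuccess and CriticalFailure to print crit damage, a failure taunt or normal damage.
; It destroys itself immediately afterward; this graph neither rolls the outcome nor applies damage.
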(event `self.ReceiveBeginPlay`
  (`parent.ReceiveBeginPlay`)
  (if (`self.Critical Success`)
    (`KismetSystemLibrary.PrintString` (`KismetStringLibrary.Concat_StrStr` "BIGGG:" (`KismetStringLibrary.Conv_IntToString` (`self.Crit Damage`))))
    (elif (`self.Critical Failure`)
      (`KismetSystemLibrary.PrintString` "Git Gud")
      (else
        (`KismetSystemLibrary.PrintString` (`KismetStringLibrary.Concat_StrStr` "Normal:" (`KismetStringLibrary.Conv_IntToString` (`self.Normal Damage`)))))))
  (`self.K2_DestroyActor`))

(fn `UserConstructionScript`
  (`parent.UserConstructionScript`))