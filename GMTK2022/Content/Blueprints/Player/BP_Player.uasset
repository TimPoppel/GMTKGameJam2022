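; BP_Player is the player combatant in what appears to be a turn-based dice game, tracking health and reporting it to the HUD.
; On start it fills health and shows the shape-shifted die from its dice component.
; TakeDamage clamps health at the maximum and, at zero or below, notifies the turn-managing actor of death.
; Attack, block and dodge events each spawn an ability actor from PlayerAbilities, passing in the player.
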(event `self.ReceiveBeginPlay`
  (set `self.Current Health` (`self.Max Health`))
  (bind _asbp_player_controller (cast `/Game/Blueprints/Player/BP_PlayerController` (`GameplayStatics.GetPlayerController` 0)))
  (bind _output_get (set `self.HUD ref` (`/Game/Blueprints/Player/BP_PlayerController.HUD ref` _asbp_player_controller)))
  (`/Game/UI/PlayerUI/BPI_HudInterface.UpdatePlayerHealth` _output_get (`self.Current Health`) (`self.Max Health`))
  (bind (_bshapeshifted _shifteddice) (`/Game/Blueprints/Components/DiceComponent/BPC_Dice.ShapeShiftDice` (`self.BPC_Dice`) 0))
  (`/Game/UI/PlayerUI/W_HUD.Get current dice` (`self.HUD ref`) _shifteddice))

(event `Take Damage`
  (params (Damage :type Integer))
  (bind _returnvalue (- (`self.Current Health`) Damage))
  (if (> Damage 0)
    (`GameplayStatics.PlaySound2D` "/Game/Sound/Player/A_Hurt_Cue.A_Hurt_Cue" 1.0 1.0 0.0 null null))
  (if (<= _returnvalue 0)
    (set `self.Current Health` _returnvalue)
    (elif (> _returnvalue (`self.Max Health`))
      (set `self.Current Health` (`self.Max Health`))
      (else
        (set `self.Current Health` _returnvalue))))
  (`/Game/UI/PlayerUI/BPI_HudInterface.UpdatePlayerHealth` (`self.HUD ref`) (`self.Current Health`) (`self.Max Health`))
  (if (<= (`self.Current Health`) 0)
    (`self.Death`)))

(event `Death`
  (bind _outactors (`GameplayStatics.GetAllActorsWithInterface` "/Game/Blueprints/TurnManager/BPI_TurnManaging.BPI_TurnManaging_C"))
  (message `/Game/Blueprints/TurnManager/BPI_TurnManaging.Died` (`|GetArrayItem` _outactors) self))

(event `/Game/Blueprints/Player/BPI_AbilitieFunctionality.Normal Attack`
  (`|SpawnActorFromClass` (`|GetArrayItem` (`self.PlayerAbilities`)) (`self.GetTransform` self) "Undefined" "OverrideRootScale" null self null))

(event `/Game/Blueprints/Player/BPI_AbilitieFunctionality.Big Attack`
  (`|SpawnActorFromClass` (`|GetArrayItem` (`self.PlayerAbilities`) 1) (`self.GetTransform` self) "Undefined" "OverrideRootScale" null self null))

(event `/Game/Blueprints/Player/BPI_AbilitieFunctionality.Blocking`
  (`|SpawnActorFromClass` (`|GetArrayItem` (`self.PlayerAbilities`) 2) (`self.GetTransform` self) "Undefined" "OverrideRootScale" null self null))

(event `/Game/Blueprints/Player/BPI_AbilitieFunctionality.Dodging`
  (`|SpawnActorFromClass` (`|GetArrayItem` (`self.PlayerAbilities`) 3) (`self.GetTransform` self) "Undefined" "OverrideRootScale" null self null))

(fn `UserConstructionScript`)