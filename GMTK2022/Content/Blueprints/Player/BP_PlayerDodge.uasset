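; BP_PlayerDodge is a short-lived player action actor that resolves a dodge in turn-based play.
; On BeginPlay it converts the roll outcome into full block plus a small heal on a critical success, full block on a high percentage, or nothing otherwise.
; It sends the result to the first actor implementing BPI_TurnManaging via PlayerActionMessage, then destroys itself.
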(event `self.ReceiveBeginPlay`
  (`parent.ReceiveBeginPlay`)
  (set `self.Block Amount` 0)
  (set `self.Healing Amount` 0)
  (if (`self.Critical Success`)
    (set `self.Block Amount` 999)
    (set `self.Healing Amount` 10)
    (elif (`self.Critical Failure`)
      (set `self.Block Amount` 0)
      (elif (> (`self.Percentage Outcome`) 0.75)
        (set `self.Block Amount` 999))))
  (`self.SendPlayerActionData` 0 (`self.Healing Amount`) (`self.Block Amount`))
  (`self.K2_DestroyActor`))

(fn `UserConstructionScript`
  (`parent.UserConstructionScript`))