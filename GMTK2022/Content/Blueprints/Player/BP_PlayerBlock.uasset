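; BP_PlayerBlock is a short-lived actor that reports the result of a player block, currently only as debug screen text.
; On BeginPlay it branches on CriticalSuccess, then CriticalFailure, printing the crit block value, a taunt, or the normal block value.
; It destroys itself immediately afterwards and applies no block effect in its own graph.
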(event `self.ReceiveBeginPlay`
  (`parent.ReceiveBeginPlay`)
  (if (`self.Critical Success`)
    (`KismetSystemLibrary.PrintString` (`KismetStringLibrary.Concat_StrStr` "BIGGG:" (`KismetStringLibrary.Conv_IntToString` (`self.Crit Block Value`))))
    (elif (`self.Critical Failure`)
      (`KismetSystemLibrary.PrintString` "Git Gud")
      (else
        (`KismetSystemLibrary.PrintString` (`KismetStringLibrary.Concat_StrStr` "Block:" (`KismetStringLibrary.Conv_IntToString` (`self.Block Value`)))))))
  (`self.K2_DestroyActor`))

(fn `UserConstructionScript`
  (`parent.UserConstructionScript`))